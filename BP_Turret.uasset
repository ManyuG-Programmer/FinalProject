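; BP_Turret is an enemy turret actor that shoots at the first-person player character and can be destroyed or hacked.
; When PawnSensing sees the player, it turns to face them, then after a short delay spawns a BP_TurretBullet from its Arrow with a sound.
; Health depletion or a hack by the player both lead to destruction with sparks and a collapse sound; hacking only prints the HackTool count beforehand.
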(event OnSeePawn(PawnSensing)
  (params (Pawn :type Pawn%20Object%20Reference))
  (Utilities|Casting|CastToBP_FirstPersonCharacter Pawn)
  (Transformation|SetActorRotation (Math|Rotator|FindLookatRotation (Transformation|GetActorLocation) (Transformation|GetActorLocation Pawn)))
  (Utilities|FlowControl|Delay 0.5)
  (Game|SpawnActorfromClass "/Game/CustomObject/Turret/BP_TurretBullet.BP_TurretBullet_C" (Transformation|GetWorldTransform (Variables|Default|GetArrow)) "Undefined" "MultiplyWithRoot" 0 0)
  (Audio|PlaySound2D "/Game/StarterContent/Audio/Explosion02.Explosion02" 1.0 1.0 0.0 0 0))

(event OnHealthDepleted(BP_HealthComponent)
  (bind _returnvalue (Transformation|GetActorLocation))
  (Actor|DestroyActor)
  (Effects|SpawnEmitteratLocation "/Game/StarterContent/Particles/P_Sparks.P_Sparks" (- _returnvalue "0.000000,0.000000,50.000000"))
  (Audio|PlaySoundatLocation "/Game/StarterContent/Audio/Collapse_Cue.Collapse_Cue" _returnvalue "0, 0, 0" 1.0 1.0 0.0 0 0 0 0))

(event EventOnHack
  (params (interactingPlayer :type Character%20Object%20Reference))
  (bind _returnvalue (Transformation|GetActorLocation))
  (bind _asbp_first_person_character (Utilities|Casting|CastToBP_FirstPersonCharacter interactingPlayer))
  (Development|PrintString (Utilities|String|Append "HackTool Amount: " (Utilities|String|ToString(Float) (Variables|/Game/FirstPerson/Blueprints/BP_FirstPersonCharacter.BP_FirstPersonCharacter_C|GethackToolAmount _asbp_first_person_character))))
  (Actor|DestroyActor)
  (Effects|SpawnEmitteratLocation "/Game/StarterContent/Particles/P_Sparks.P_Sparks" (- _returnvalue "0.000000,0.000000,50.000000"))
  (Audio|PlaySoundatLocation "/Game/StarterContent/Audio/Collapse_Cue.Collapse_Cue" _returnvalue "0, 0, 0" 1.0 1.0 0.0 0 0 0 0))

(event EventBeginPlay
  (Variables|/Game/CustomBlueprint/BP_HealthComponent.BP_HealthComponent_C|SetMaxHealth (Variables|Default|GetBP_HealthComponent) 1e+02))

(fn ConstructionScript)