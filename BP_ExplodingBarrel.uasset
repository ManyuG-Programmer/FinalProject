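; BP_ExplodingBarrel is a barrel actor that explodes when its health component is depleted.
; A hit while the barrel moves fast enough applies self-damage equal to max health, provided the first-person character's ExplodeObject flag is set.
; On depletion, a DoOnce-guarded sequence deals full radial damage, fires a RadialForce impulse, destroys the actor and spawns explosion particles and sound.
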(event OnHealthDepleted(BP_HealthComponent)
  (bind _returnvalue (Transformation|GetActorLocation))
  (Utilities|FlowControl|DoOnce false
    (:Completed
      (Game|Damage|ApplyRadialDamage 1e+02 (Transformation|GetActorLocation) 5e+02 0 0 self 0 true "ECC_Visibility")
      (Class|RadialForceComponent|FireImpulse (Variables|Default|GetRadialForce))
      (Actor|DestroyActor)
      (Effects|SpawnEmitteratLocation "/Game/StarterContent/Particles/P_Explosion.P_Explosion" _returnvalue "0, 0, 0" "3.000000,3.000000,3.000000")
      (Audio|PlaySoundatLocation "/Game/StarterContent/Audio/Explosion01.Explosion01" _returnvalue "0, 0, 0" 1.0 1.0 0.0 0 0 0 0))))

(event OnComponentHit(Barrel)
  (params (HitComponent :type Primitive%20Component%20Object%20Reference) (OtherActor :type Actor%20Object%20Reference) (OtherComp :type Primitive%20Component%20Object%20Reference) (NormalImpulse :type Vector :default "0, 0, 0") (Hit :type Hit%20Result%20Structure%20%28by%20ref%29))
  (bind _returnvalue (Actor|GetActorOfClass "/Game/FirstPerson/Blueprints/BP_FirstPersonCharacter.BP_FirstPersonCharacter_C"))
  (if (and (Variables|/Game/FirstPerson/Blueprints/BP_FirstPersonCharacter.BP_FirstPersonCharacter_C|GetexplodeObject _returnvalue) (> (Math|Vector|VectorLength (Transformation|GetComponentVelocity (Variables|Default|GetBarrel))) 1e+02))
    (Game|Damage|ApplyDamage self (Variables|/Game/CustomBlueprint/BP_HealthComponent.BP_HealthComponent_C|GetMaxHealth (Variables|Default|GetBP_HealthComponent)) 0 0)))

(fn ConstructionScript)