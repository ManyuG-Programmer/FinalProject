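; BP_Generator is a generator actor whose destruction also destroys every BP_Turret in the level.
; It can fall either to repeated hacking, counted in OnHack until the third hack, or to its health component depleting.
; Health depletion also spawns a spark emitter and plays a collapse sound, while a hack takedown has no effects.
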(event OnHealthDepleted(BP_HealthComponent)
  (bind _returnvalue (Transformation|GetActorLocation))
  (Actor|DestroyActor)
  (Effects|SpawnEmitteratLocation "/Game/StarterContent/Particles/P_Sparks.P_Sparks" (- _returnvalue "0.000000,0.000000,50.000000"))
  (Audio|PlaySoundatLocation "/Game/StarterContent/Audio/Collapse_Cue.Collapse_Cue" _returnvalue "0, 0, 0" 1.0 1.0 0.0 0 0 0 0)
  (bind _outactors (Actor|GetAllActorsOfClass "/Game/CustomObject/Turret/BP_Turret.BP_Turret_C"))
  (Actor|DestroyActor _outactors))

(event EventBeginPlay
  (Variables|/Game/CustomBlueprint/BP_HealthComponent.BP_HealthComponent_C|SetMaxHealth (Variables|Default|GetBP_HealthComponent) 1e+02))

(event EventOnHack
  (params (interactingPlayer :type Character%20Object%20Reference))
  (Development|PrintString (Utilities|String|ToString(Float) (Variables|Default|GethackCount)))
  (Variables|Default|SethackCount (+ (Variables|Default|GethackCount) 1.0))
  (if (> (Variables|Default|GethackCount) 2.0)
    (Actor|DestroyActor)
    (bind _outactors (Actor|GetAllActorsOfClass "/Game/CustomObject/Turret/BP_Turret.BP_Turret_C"))
    (Actor|DestroyActor _outactors)))

(fn ConstructionScript)